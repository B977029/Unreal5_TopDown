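; BP_Player is the player pawn, a sprite-based 2D character driven by Enhanced Input for moving and attacking.
; On BeginPlay it adds the player mapping context and caches BP_PlayerState, whose WorldMoveVector supplies the movement axes.
; Move input records direction and flips the sprite by horizontal sign, restoring the idle flipbook on release.
; Attack input blocks movement until completed and jumps the animation instance to its attack node.
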(event Input|EnhancedActionEvents|EnhancedInputActionIA_PlayerMove
  (params (ActionValue :type Vector%202D%20Structure) (ElapsedSeconds :type Float%20%28double-precision%29) (TriggeredSeconds :type Float%20%28double-precision%29) (InputAction :type Input%20Action%20Object%20Reference :default "/Game/BulePrint/IA_PlayerMove.IA_PlayerMove"))
  (bind _as_bp_player_state (Variables|Default|GetAs%20BP%20Player%20State))
  (bind _sprite (Variables|Default|GetSprite))
  (bind _worldmovevector (Variables|/Game/BulePrint/BP_PlayerState.BP_PlayerState_C|GetWorldMoveVector _as_bp_player_state))
  (:Triggered
    (if (Variables|Default|GetCanMove)
      (Utilities|FlowControl|Sequence
        (:then_0
          (Pawn|Input|AddMovementInput (Math|Vector|MakeVector (.x _worldmovevector) 0.0 0.0) (.x ActionValue) false)
          (Pawn|Input|AddMovementInput (Math|Vector|MakeVector 0.0 (.y _worldmovevector) 0.0) (.y ActionValue) false)
          (Variables|Default|SetDirection (Math|Vector2D|MakeVector2D (.x ActionValue) (.y ActionValue))))
        (:then_1
          (if (> (.x ActionValue) 0.0)
            (Transformation|SetWorldRotation _sprite "0.000000,0.000000,-90.000000" false false)
            (else
              (Transformation|SetWorldRotation _sprite "-180.000000,0.000000,-90.000000" false false)))))))
  (:Started
    (Variables|Default|SetIsMove true))
  (:Completed
    (Variables|Default|SetIsMove false)
    (Sprite|SetFlipbook _sprite "/Game/Art/Player/PB_Player_IdleR.PB_Player_IdleR")))

(event Input|EnhancedActionEvents|EnhancedInputActionIA_PlayerAttack
  (params (ActionValue :type Boolean) (ElapsedSeconds :type Float%20%28double-precision%29) (TriggeredSeconds :type Float%20%28double-precision%29) (InputAction :type Input%20Action%20Object%20Reference :default "/Game/BulePrint/IA_PlayerAttack.IA_PlayerAttack"))
  (:Triggered
    (Variables|Default|SetIsAttack true)
    (Variables|Default|SetCanMove false)
    (Class|PaperZDAnimInstance|JumptoNode (Variables|/Script/PaperZD.PaperZDAnimationComponent|GetAnimInstance (Variables|Default|GetAnimationComponent)) "Jump_Attack" "None"))
  (:Completed
    (Variables|Default|SetIsAttack false)
    (Variables|Default|SetCanMove true)))

(event EventBeginPlay
  (Utilities|FlowControl|Sequence
    (:then_0
      (Utilities|FlowControl|Sequence
        (:then_0
          (bind _asplayer_controller (Utilities|Casting|CastToPlayerController (Pawn|GetController)))
          (Input|AddMappingContext (PlayerController|LocalPlayerSubsystems|GetEnhancedInputLocalPlayerSubsystem _asplayer_controller) "/Game/BulePrint/IMC_Player.IMC_Player" 0 "(bIgnoreAllPressedKeysUntilRelease=True,bForceImmediately=False)"))
        (:then_1
          (bind _asbp_player_state (Utilities|Casting|CastToBP_PlayerState (Game|GetPlayerState 0)))
          (Variables|Default|SetAs%20BP%20Player%20State _asbp_player_state))))))

(event Collision|EventActorBeginOverlap
  (params (OtherActor :type Actor%20Object%20Reference)))

(event EventTick
  (params (DeltaSeconds :type Float%20%28single-precision%29)))

(fn ConstructionScript)