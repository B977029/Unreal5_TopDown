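; BP_Slime is a slime enemy that takes hits, dies and rewards the player.
; BeginPlay caches the player state, main game mode and its UI_Slime widget.
; Hitted subtracts damage via the player state's Damege call, displays it on the widget and jumps animation nodes to hit or death.
; Death waits briefly, grants experience and gold, destroys the actor and requests a respawn at its Spot from the game mode.
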(event Custom|Hitted
  (bind _animationcomponent (Variables|Default|GetAnimationComponent))
  (bind _animinstance (Variables|/Script/PaperZD.PaperZDAnimationComponent|GetAnimInstance _animationcomponent))
  (bind _output_get (Default|Damege (Variables|Default|GetAs%20BP%20Player%20State)))
  (Variables|Default|SetHP (- (Variables|Default|GetHP) _output_get))
  (Default|ShowDamage (Variables|Default|GetAs%20UI%20Slime) _output_get)
  (if (<= (Variables|Default|GetHP) 0)
    (Class|PaperZDAnimInstance|JumptoNode _animinstance "Jump_Die" "None")
    (Utilities|FlowControl|Delay 0.2)
    (CallFunction|Dead)
    (else
      (Class|PaperZDAnimInstance|JumptoNode _animinstance "Jump_Hitted" "None"))))

(event Custom|Dead
  (Default|ExpUp (Variables|Default|GetAs%20BP%20Player%20State) (Variables|Default|GetD_Exp))
  (CallFunction|Drop)
  (Actor|DestroyActor)
  (Default|RespawnSlime (Variables|Default|GetAs%20BP%20Game%20Mode%20Main) (Variables|Default|GetSpot)))

(event Custom|Drop
  (Default|GoldUp (Variables|Default|GetAs%20BP%20Player%20State) (Variables|Default|GetD_Gold)))

(event EventBeginPlay
  (Utilities|FlowControl|Sequence
    (:then_0
      (bind _asbp_player_state (Utilities|Casting|CastToBP_PlayerState (Game|GetPlayerState 0)))
      (Variables|Default|SetAs%20BP%20Player%20State _asbp_player_state))
    (:then_1
      (bind _asbp_game_mode_main (Utilities|Casting|CastToBP_GameMode_Main (Game|GetGameMode)))
      (Variables|Default|SetAs%20BP%20Game%20Mode%20Main _asbp_game_mode_main))
    (:then_2
      (bind _asui_slime (Utilities|Casting|CastToUI_Slime (UserInterface|GetWidget (Variables|Default|GetWidget))))
      (Variables|Default|SetAs%20UI%20Slime _asui_slime))))

(event Collision|EventActorBeginOverlap
  (params (OtherActor :type Actor%20Object%20Reference)))

(event EventTick
  (params (DeltaSeconds :type Float%20%28single-precision%29)))

(fn ConstructionScript)