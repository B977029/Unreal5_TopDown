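; BP_PlayerState is a player stats Blueprint that holds experience, level, gold, speed and a movement vector.
; BeginPlay scales the X and Y of WorldMoveVector by Speed and zeroes Z.
; LevelUp sets Exp to Level plus one and raises MaxExp, leaving Level itself unchanged.
; ExpUp and GoldUp functions add an amount to their totals, but their same-named events pass zero.
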(event Custom|LevelUp
  (Variables|Default|SetExp (+ (Variables|Default|GetLevel) 1))
  (Variables|Default|SetMaxExp (+ (Variables|Default|GetMaxExp) 10)))

(event Custom|ExpUp
  (CallFunction|ExpUp))

(event Custom|GoldUp
  (CallFunction|GoldUp))

(event EventBeginPlay
  (Utilities|FlowControl|Sequence
    (:then_0
      (Variables|Default|SetWorldMoveVector (Math|Vector|MakeVector (* (Variables|Default|GetSpeed) (.x (Variables|Default|GetWorldMoveVector))) (* (Variables|Default|GetSpeed) (.y (Variables|Default|GetWorldMoveVector))) 0.0)))))

(event EventTick
  (params (DeltaSeconds :type Float%20%28single-precision%29)))

(fn ConstructionScript)

(fn ExpUp
  (params (B :type Integer))
  (Variables|Default|SetExp (+ (Variables|Default|GetExp) B)))

(fn GoldUp
  (params (B :type Integer))
  (Variables|Default|SetGold (+ (Variables|Default|GetGold) B)))